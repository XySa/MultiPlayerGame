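; Game instance Blueprint that handles LAN multiplayer sessions: creating, listing and joining games, plus printing session, network and travel errors.
; CreateGame hosts a session and opens Lvl1 as a listen server.
; GetGames sends each found session's details to WBP_MainMenu, but obtains it by casting the game instance, so that cast likely fails.
; JoinGame runs its own search and calls JoinSession on every result, with no selection.
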(event Custom|CreateGame
  ;[1 1 1] Create Game Session
  (|Session (Game|GetPlayerController 0) 16 true
    (:OnSuccess
      (Game|OpenLevel(byName) "Lvl1" true "listen"))
    (:OnFailure
      (Development|PrintString "Faild Create session"))))

(event Custom|JoinGame
  (bind _returnvalue (Game|GetPlayerController 0))
  ;[1 1 1] Join game
  (bind _results (|FindSessions _returnvalue 20 true)
    (:OnSuccess
      (for _array_element _results
        (|JoinSession _returnvalue _array_element
          (:OnFailure
            (Development|PrintString "Join session failed")))))
    (:OnFailure
      (Development|PrintString "Game joining failed"))))

(event Custom|GetGames
  ;[1 1 1] Find Game
  (bind _results (|FindSessions (Game|GetPlayerController 0) 20 true)
    (:OnSuccess
      (for _array_element _results
        (bind _aswbp_main_menu (Utilities|Casting|CastToWBP_MainMenu (Game|GetGameInstance)))
        (Default|AddDatatoList _aswbp_main_menu (Utilities|Struct|MakeSData (Class|FindSessionsCallbackProxy|GetServerName _array_element) (Utilities|String|ToString(Integer) (Class|FindSessionsCallbackProxy|GetCurrentPlayers _array_element)) (Utilities|String|ToString(Integer) (Class|FindSessionsCallbackProxy|GetMaxPlayers _array_element)) (Utilities|String|ToString(Integer) (Class|FindSessionsCallbackProxy|GetPinginMs _array_element))))))
    (:OnFailure
      (Development|PrintString "Game search failed"))))

(event EventHandleNetworkError
  (params (FailureType :type ENetworkFailure%20Enum :default "NetDriverAlreadyExists") (bIsServer :type Boolean))
  ;[1 1 1] Network
  (Development|PrintString (Utilities|String|Append "Network eror:" (Utilities|String|EnumtoString FailureType) "on server?" (Utilities|String|ToString(Boolean) bIsServer))))

(event EventHandleTravelError
  (params (FailureType :type ETravelFailure%20Enum :default "NoLevel"))
  ;[1 1 1] Network
  (Development|PrintString (Utilities|String|EnumtoString FailureType)))