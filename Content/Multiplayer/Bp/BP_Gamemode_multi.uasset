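; Multiplayer game mode that sorts joining players into two teams.
; On PostLogin it casts the new player to Bp_PlayerControllerMulti and puts it on whichever team array is smaller, with ties going to team 1, then sets its team ID.
; A failed cast only prints a message, and the logout handler is empty, so the game mode does not remove departing players from the arrays.
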(event EventBeginPlay)

(event EventTick
  (params (DeltaSeconds :type Float%20%28single-precision%29)))

(event EventPostLogin
  (params (NewPlayer :type Player%20Controller%20Object%20Reference))
  (bind _asbp_player_controller_multi (Utilities|Casting|CastToBp_PlayerControllerMulti NewPlayer)
    (:then
      (if (< (Utilities|Array|Length (Variables|Default|GetTeam2)) (Utilities|Array|Length (Variables|Default|GetTeam1)))
        (Default|SetTeamID _asbp_player_controller_multi 2)
        (Utilities|Array|Add (Variables|Default|GetTeam2) _asbp_player_controller_multi)
        (else
          (Default|SetTeamID _asbp_player_controller_multi 1)
          (Utilities|Array|Add (Variables|Default|GetTeam1) _asbp_player_controller_multi))))
    (:CastFailed
      (Development|PrintString "Failed to cast"))))

(event EventOnLogout
  (params (ExitingController :type Controller%20Object%20Reference)))

(fn ConstructionScript)