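; Multiplayer projectile that flies forward, damages characters it overlaps and destroys itself on impact or when its lifetime timer expires.
; The server moves it each Tick by setting its location without sweep, so hits come from the sphere's overlap event, also handled on the server.
; Collisions ignore the owner and other projectiles; any other hit triggers a multicast emitter effect and destruction, with damage applied only to BP_Charater_multi.
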(event OnComponentBeginOverlap(Sphere)
  (params (OverlappedComponent :type Primitive%20Component%20Object%20Reference) (OtherActor :type Actor%20Object%20Reference) (OtherComp :type Primitive%20Component%20Object%20Reference) (OtherBodyIndex :type Integer) (bFromSweep :type Boolean) (SweepResult :type Hit%20Result%20Structure%20%28by%20ref%29))
  (if (Networking|IsServer)
    (CallFunction|ServerCollision OtherActor (Transformation|GetActorLocation))))

(event Custom|LifeEnded
  (CallFunction|ServerLifeEnded))

(event Custom|Server_LifeEnded
  (Actor|DestroyActor))

(event Custom|ServerMove
  (params (Delta%20time :type Float%20%28single-precision%29))
  (Transformation|SetActorLocation (+ (Transformation|GetActorLocation) (* (Transformation|GetActorForwardVector) (* Delta%20time (Variables|Default|Getspeed)))) false false))

(event Custom|Server_collision
  (params (Actor :type Actor%20Object%20Reference) (Loaction :type Vector))
  (if (!= Actor (Components|GetOwner))
    (bind _asbp_charater_multi (Utilities|Casting|CastToBP_Charater_multi Actor)
      (:then
        (Default|ServerTakeDamage _asbp_charater_multi (Variables|Default|GetDamage)))
      (:CastFailed
        (Utilities|Casting|CastToBP_Projectile Actor
          (:CastFailed
            _))))
    (CallFunction|MulticastHitEvent Loaction)
    (CallFunction|ServerLifeEnded)))

(event Custom|SpawnHiteff
  (params (location :type Vector))
  (Effects|SpawnEmitteratLocation 0 location))

(event Custom|Multicast%20hit%20event
  (params (location :type Vector))
  (CallFunction|SpawnHiteff location))

(event EventBeginPlay
  (Utilities|Time|SetTimerbyEvent (delegate Custom|LifeEnded) (Variables|Default|GetTTL)))

(event Collision|EventActorBeginOverlap
  (params (OtherActor :type Actor%20Object%20Reference)))

(event EventTick
  (params (DeltaSeconds :type Float%20%28single-precision%29))
  (if (Networking|IsServer)
    (CallFunction|ServerMove DeltaSeconds)))

(fn ConstructionScript)